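; Monster enemy Blueprint that hunts and attacks the player's BP_Knight, running a simple state machine every Tick.
; Idle looks up the knight with GetActorOfClass and switches to Move once it is valid, with no proximity check.
; Move calls AttackBegin inside a hardcoded range, otherwise sets a four-way Direction along the dominant X or Z axis toward the target.
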(event `self.ReceiveTick`
  (params (DeltaSeconds :type "Float (single-precision)"))
  (`parent.ReceiveTick` DeltaSeconds)
  (`self.AI`))

(event `self.ReceiveBeginPlay`
  (`parent.ReceiveBeginPlay`))

(fn `AI`
  (bind _targetenemy (`self.TargetEnemy`))
  (bind (_chasedirectionvector_x _chasedirectionvector_y _chasedirectionvector_z) (`KismetMathLibrary.BreakVector` (`self.ChaseDirectionVector`)))
  (switch `/Game/BluePrint/EnumState` (`self.State`) ; 매 프레임마다 관리
    (:`NewEnumerator0`
      (bind _returnvalue (`GameplayStatics.GetActorOfClass` "/Game/BluePrint/BP_Knight.BP_Knight_C"))
      (bind _output_get (set `self.TargetEnemy` _returnvalue))
      (`/Engine/EditorBlueprintResources/StandardMacros.IsValid` _output_get ; 플레이어가 주변에 있는가?
        (:`Is Valid`
          (set `self.State` "NewEnumerator1"))))
    (:`NewEnumerator1`
      (`/Engine/EditorBlueprintResources/StandardMacros.IsValid` _targetenemy
        (:`Is Valid`
          (bind _output_get_2 (set `self.ChaseDirectionVector` (- (`self.K2_GetActorLocation` _targetenemy) (`self.K2_GetActorLocation`)))) ; 방향벡터 구하기
          (if (< (`KismetMathLibrary.VSize` _output_get_2) 300.0)
            (`self.Attack_Begin`) ; 사정거리에 들어왔을때 플레이어를 공격
            (elif (> (`KismetMathLibrary.Abs` _chasedirectionvector_x) (`KismetMathLibrary.Abs` _chasedirectionvector_z))
              (`/Engine/EditorBlueprintResources/StandardMacros.CompareFloat` _chasedirectionvector_x ; 좌우이동
                (:`>`
                  (set `self.Direction` "NewEnumerator3"))
                (:`<`
                  (set `self.Direction` "NewEnumerator2")))
              (else
                (`/Engine/EditorBlueprintResources/StandardMacros.CompareFloat` _chasedirectionvector_z ; 위아래이동
                  (:`>`
                    (set `self.Direction` "NewEnumerator0"))
                  (:`<`
                    (set `self.Direction` "NewEnumerator1")))))))))))

(fn `UserConstructionScript`
  (`parent.UserConstructionScript`))