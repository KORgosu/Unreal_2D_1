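; AI controller for BP_Monster that makes it target the player's BP_Knight and attack it at close range.
; On possess it caches the monster, then every tick runs a state machine on the monster's State.
; Idle targets a BP_Knight found by class lookup and switches to Move.
; Move waits until the monster arrives, turns it toward the target, and begins an attack when exactly one tile away.
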(event `self.ReceivePossess`
  (params (PossessedPawn :type "Pawn Object Reference"))
  (bind _asbp_monster (cast `/Game/BluePrint/Creatures/BP_Monster` PossessedPawn))
  (set `self.Monster1` _asbp_monster))

(event `self.ReceiveTick`
  (params (DeltaSeconds :type "Float (single-precision)"))
  (`self.Update AI`))

(fn `Update AI`
  (bind _monster1 (`self.Monster1`))
  (bind _monster1_2 (`self.Monster1`))
  (bind _targetenemy (`/Game/BluePrint/Creatures/BP_Monster.TargetEnemy` _monster1))
  (switch `/Game/BluePrint/EnumStruct/EnumState` (`/Game/BluePrint/Creatures/BP_Creature.State` _monster1) ; 매 프레임마다 관리
    (:`NewEnumerator0`
      (bind _returnvalue (`GameplayStatics.GetActorOfClass` "/Game/BluePrint/Creatures/BP_Knight.BP_Knight_C"))
      (bind _output_get (set `/Game/BluePrint/Creatures/BP_Monster.TargetEnemy` _returnvalue (`self.Monster1`)))
      (`/Engine/EditorBlueprintResources/StandardMacros.IsValid` _output_get ; 플레이어가 주변에 있는가?
        (:`Is Valid`
          (set `/Game/BluePrint/Creatures/BP_Creature.State` "NewEnumerator1" (`self.Monster1`)))))
    (:`NewEnumerator1`
      (`/Engine/EditorBlueprintResources/StandardMacros.IsValid` _targetenemy
        (:`Is Valid`
          (if (`/Game/BluePrint/Creatures/BP_Creature.ArrivedToDestination` _monster1)
            (`/Game/BluePrint/Creatures/BP_Creature.LookTarget` _monster1_2 _targetenemy)
            (bind _count (`/Game/BluePrint/Creatures/BP_Creature.GetTileCount` _monster1_2 _targetenemy)) ; 한칸이 남았을 경우 공격
            (if (== _count 1)
              (`/Game/BluePrint/Creatures/BP_Creature.Attack_Begin` (`self.Monster1`)) ; 사정거리에 들어왔을때 플레이어를 공격
            )))))))

(fn `UserConstructionScript`)