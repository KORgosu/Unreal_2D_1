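; Player controller that turns movement input into state and facing direction for the controlled BP_Knight.
; BeginPlay caches the knight, and every Tick runs InputUpdate, which acts only while the knight is Idle or Move.
; Any non-zero up or right axis sets Move, otherwise Idle, and the axis signs pick one of four Direction values.
; Horizontal input is evaluated last, so it overrides vertical on diagonals.
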(event `self.ReceiveBeginPlay`
  (bind _asbp_knight (cast `/Game/BluePrint/Creatures/BP_Knight` (`self.K2_GetPawn`)))
  (set `self.As BP Knight` _asbp_knight))

(event `self.ReceiveTick`
  (params (DeltaSeconds :type "Float (single-precision)"))
  (`self.Input Update`))

(fn `Input Update`
  (bind _as_bp_knight (`self.As BP Knight`))
  (switch `/Game/BluePrint/EnumStruct/EnumState` (`/Game/BluePrint/Creatures/BP_Creature.State` (`self.As BP Knight`))
    (:`NewEnumerator0`
      _)
    (:`NewEnumerator1`
      _))
  (`|ExecutionSequence`
    (:`then_0`
      (if (or (!= (`self.GetInputAxisValue`) 0.0) (!= (`self.GetInputAxisValue`) 0.0))
        (set `/Game/BluePrint/Creatures/BP_Creature.State` "NewEnumerator1" _as_bp_knight)
        (else
          (set `/Game/BluePrint/Creatures/BP_Creature.State` "NewEnumerator0" _as_bp_knight))))
    (:`then_1`
      (`/Engine/EditorBlueprintResources/StandardMacros.CompareFloat` (`self.GetInputAxisValue`)
        (:`>`
          (set `/Game/BluePrint/Creatures/BP_Creature.Direction` "NewEnumerator0" _as_bp_knight))
        (:`<`
          (set `/Game/BluePrint/Creatures/BP_Creature.Direction` "NewEnumerator1" _as_bp_knight))))
    (:`then_2`
      (`/Engine/EditorBlueprintResources/StandardMacros.CompareFloat` (`self.GetInputAxisValue`)
        (:`>`
          (set `/Game/BluePrint/Creatures/BP_Creature.Direction` "NewEnumerator3" _as_bp_knight))
        (:`<`
          (set `/Game/BluePrint/Creatures/BP_Creature.Direction` "NewEnumerator2" _as_bp_knight))))))

(fn `UserConstructionScript`)