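; Knight creature Blueprint, a child class that leaves most behavior to its parent.
; On BeginPlay it stores the "Knight" row of the creature data table in Data, and runs the parent BeginPlay only if that row is found.
; The Attack input calls AttackBegin, and Tick just forwards to the parent.
; The remaining function, macro and debug text nodes are empty or unused leftovers.
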(event `self.ReceiveTick`
  (params (DeltaSeconds :type "Float (single-precision)"))
  (`parent.ReceiveTick` DeltaSeconds))

(event `InputAction|Attack`
  (params (Key :type "Key Structure"))
  (:`Pressed`
    (`self.Attack_Begin`)))

(event `self.ReceiveBeginPlay`
  (bind _returnvalue (`|GetDataTableRow` "/Game/BluePrint/DataTable/Creature_DataTable.Creature_DataTable" "Knight")
    (:`then`
      (set `self.Data` _returnvalue)
      (`parent.ReceiveBeginPlay`))))

(fn `UserConstructionScript`)

(fn `새 함수_0_0`)