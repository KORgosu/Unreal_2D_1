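; Grid-based 2D creature that moves tile by tile, melee attacks and takes damage, with stats and flipbooks read from Data.
; Tick runs movement toward the current cell, querying BP_TileMap for the next walkable one on arrival, then picks the flipbook from State and Direction.
; Attacks damage the creature in the faced adjacent cell, and OnDamaged updates the HP bar widget.
; Helpers give Manhattan tile distance and turn toward a target along its farther axis.
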(event `self.ReceiveBeginPlay`
  (bind _output_get (set `self.HP` (`.HPMAX_26_8AC06505446583406658AEB219CB0C5F` (break `/Game/BluePrint/DataTable/Creature_Data` (`self.Data`)))))
  (set `self.MaxHP` _output_get))

(event `self.ReceiveTick`
  (params (DeltaSeconds :type "Float (single-precision)"))
  (`self.Update Logic`)
  (`self.Update Animate`))

(event `Attack_Begin`
  (switch `/Game/BluePrint/EnumStruct/EnumState` (`self.State`)
    (:`NewEnumerator0`
      _)
    (:`NewEnumerator1`
      _))
  (set `self.State` "NewEnumerator2")
  (`self.Update Animate`)
  (`self.Attack_Process`)
  (`KismetSystemLibrary.Delay` (`PaperFlipbookComponent.GetFlipbookLength` (`self.Sprite`)))
  (set `self.State` "NewEnumerator1"))

(fn `ArrivedToDestination`
  (returns (HasArrived :type Boolean))
  (return (<= (`KismetMathLibrary.VSize` (- (`self.CharcterPos`) (`self.K2_GetActorLocation`))) 10.0)))

(fn `Attack_Process`
  (bind (_gridpos_x _gridpos_y) (break `/Game/BluePrint/EnumStruct/EnumGridPosition` (`self.GridPos`)))
  (bind (_data_hpmax _data_damage) (break `/Game/BluePrint/DataTable/Creature_Data` (`self.Data`)))
  (bind (_returnvalue_x _returnvalue_y) (break `/Game/BluePrint/EnumStruct/EnumGridPosition` (select `/Game/BluePrint/EnumStruct/EnumDirection` (`self.Direction`) :`NewEnumerator0` (make `/Game/BluePrint/EnumStruct/EnumGridPosition` 0 -1) :`NewEnumerator1` (make `/Game/BluePrint/EnumStruct/EnumGridPosition` 0 1) :`NewEnumerator2` (make `/Game/BluePrint/EnumStruct/EnumGridPosition` -1) :`NewEnumerator3` (make `/Game/BluePrint/EnumStruct/EnumGridPosition` 1) :!type "/Game/BluePrint/EnumStruct/EnumGridPosition Structure")))
  (bind _returnvalue (`GameplayStatics.GetActorOfClass` "/Game/BluePrint/BP_TileMap.BP_TileMap_C"))
  (bind (_isfound _creature) (`/Game/BluePrint/BP_TileMap.GetCreatureAtGrid` _returnvalue (+ _gridpos_x _returnvalue_x) (+ _gridpos_y _returnvalue_y))) ; 다음좌표에 뭐가 있는가?
  (if _isfound
    (`self.OnDamaged` _creature _data_damage self)))

(fn `GetTileCount`
  (params (Target :type "/Game/BluePrint/Creatures/BP_Creature Object Reference"))
  (returns (Count :type Integer))
  (bind (_gridpos_x _gridpos_y) (break `/Game/BluePrint/EnumStruct/EnumGridPosition` (`/Game/BluePrint/Creatures/BP_Creature.GridPos` Target)))
  (bind (_gridpos_x_2 _gridpos_y_2) (break `/Game/BluePrint/EnumStruct/EnumGridPosition` (`self.GridPos`)))
  (return (+ (`KismetMathLibrary.Abs_Int` (- _gridpos_x _gridpos_x_2)) (`KismetMathLibrary.Abs_Int` (- _gridpos_y _gridpos_y_2)))) ; 반환되는 값은 칸 수
)

(fn `LookTarget`
  (params (Target :type "/Game/BluePrint/Creatures/BP_Creature Object Reference"))
  (locals (DiffX :type Integer) (DiffY :type Integer))
  (bind (_gridpos_x _gridpos_y) (break `/Game/BluePrint/EnumStruct/EnumGridPosition` (`/Game/BluePrint/Creatures/BP_Creature.GridPos` Target)))
  (bind (_gridpos_x_2 _gridpos_y_2) (break `/Game/BluePrint/EnumStruct/EnumGridPosition` (`self.GridPos`)))
  (bind _diffx (`local.DiffX`))
  (bind _diffy (`local.DiffY`))
  (`/Engine/EditorBlueprintResources/StandardMacros.IsValid` Target
    (:`Is Valid`
      (set `local.DiffX` (- _gridpos_x _gridpos_x_2))
      (set `local.DiffY` (- _gridpos_y _gridpos_y_2))
      (if (>= (`KismetMathLibrary.Abs_Int` _diffx) (`KismetMathLibrary.Abs_Int` _diffy))
        (`/Engine/EditorBlueprintResources/StandardMacros.CompareInt` _diffx
          (:`>`
            (set `self.Direction` "NewEnumerator3"))
          (:`<`
            (set `self.Direction` "NewEnumerator2")))
        (else
          (`/Engine/EditorBlueprintResources/StandardMacros.CompareInt` _diffy
            (:`>`
              (set `self.Direction` "NewEnumerator1"))
            (:`<`
              (set `self.Direction` "NewEnumerator0"))))))))

(fn `OnDamaged`
  (params (Damage :type Integer) (Attack :type "/Game/BluePrint/Creatures/BP_Creature Object Reference"))
  (bind _maxhp (`self.MaxHP`))
  (if (not (== Attack self))
    (bind _output_get (set `self.HP` (`KismetMathLibrary.Clamp` (- (`self.HP`) Damage) 0 _maxhp)))
    (bind _aswizet_bp_hp (cast `/Game/BluePrint/UI/WizetBP_HP` (`WidgetComponent.GetUserWidgetObject` (`self.HpBar`))))
    (set `/Game/BluePrint/UI/WizetBP_HP.HpRatio` (/ _output_get (`KismetMathLibrary.Conv_IntToDouble` _maxhp)) _aswizet_bp_hp)))

(fn `SettingCharPos`
  (params (GridX :type Integer) (GridY :type Integer) (ForceMove :type Boolean))
  (bind (_returnvalue_x _returnvalue_y) (`KismetMathLibrary.BreakVector` (`self.K2_GetActorLocation`)))
  (bind _returnvalue (`GameplayStatics.GetActorOfClass` "/Game/BluePrint/BP_TileMap.BP_TileMap_C"))
  (bind (_valid _pos) (`/Game/BluePrint/BP_TileMap.GetWorldPos` _returnvalue GridX GridY))
  (if _valid
    (set `self.GridPos` (make `/Game/BluePrint/EnumStruct/EnumGridPosition` GridX GridY))
    (bind _output_get (set `self.CharcterPos` (`KismetMathLibrary.MakeVector` (.x _pos) _returnvalue_y (.z _pos))))
    (if ForceMove
      (`self.K2_SetActorLocation` _output_get))))

(fn `Update Animate`
  (bind (_data_hpmax _data_damage _data_up_idle _data_down_idle _data_side_idle _data_up_move _data_down_move _data_side_move _data_up_attack _data_down_attack _data_side_attack) (break `/Game/BluePrint/DataTable/Creature_Data` (`self.Data`)))
  (`SceneComponent.K2_SetRelativeRotation` (`self.Sprite`) (select `bool` (`|EnumEquality` (`self.Direction`) "NewEnumerator2") :`true` (struct :`Yaw` 180.0) :!type "Rotator Structure") false false)
  (switch `/Game/BluePrint/EnumStruct/EnumState` (`self.State`)
    (:`NewEnumerator0`
      (`PaperFlipbookComponent.SetFlipbook` (`self.Sprite`) (select `/Game/BluePrint/EnumStruct/EnumDirection` (`self.Direction`) :`NewEnumerator0` _data_up_idle :`NewEnumerator1` _data_down_idle :`NewEnumerator2` _data_side_idle :`NewEnumerator3` _data_side_idle)))
    (:`NewEnumerator1`
      (`PaperFlipbookComponent.SetFlipbook` (`self.Sprite`) (select `/Game/BluePrint/EnumStruct/EnumDirection` (`self.Direction`) :`NewEnumerator0` _data_up_move :`NewEnumerator1` _data_down_move :`NewEnumerator2` _data_side_move :`NewEnumerator3` _data_side_move)))
    (:`NewEnumerator2`
      (`PaperFlipbookComponent.SetFlipbook` (`self.Sprite`) (select `/Game/BluePrint/EnumStruct/EnumDirection` (`self.Direction`) :`NewEnumerator0` _data_up_attack :`NewEnumerator1` _data_down_attack :`NewEnumerator2` _data_side_attack :`NewEnumerator3` _data_side_attack)))))

(fn `Update Destination`
  (bind (_gridpos_x _gridpos_y) (break `/Game/BluePrint/EnumStruct/EnumGridPosition` (`self.GridPos`)))
  (bind (_returnvalue_x _returnvalue_y) (break `/Game/BluePrint/EnumStruct/EnumGridPosition` (select `/Game/BluePrint/EnumStruct/EnumDirection` (`self.Direction`) :`NewEnumerator0` (make `/Game/BluePrint/EnumStruct/EnumGridPosition` 0 -1) :`NewEnumerator1` (make `/Game/BluePrint/EnumStruct/EnumGridPosition` 0 1) :`NewEnumerator2` (make `/Game/BluePrint/EnumStruct/EnumGridPosition` -1) :`NewEnumerator3` (make `/Game/BluePrint/EnumStruct/EnumGridPosition` 1) :!type "/Game/BluePrint/EnumStruct/EnumGridPosition Structure")))
  (bind _returnvalue (+ _gridpos_x _returnvalue_x))
  (bind _returnvalue_2 (+ _gridpos_y _returnvalue_y))
  (if (not (`self.StopMove`))
    (bind _returnvalue_3 (`GameplayStatics.GetActorOfClass` "/Game/BluePrint/BP_TileMap.BP_TileMap_C"))
    (bind _go (`/Game/BluePrint/BP_TileMap.Go` _returnvalue_3 _returnvalue _returnvalue_2)) ; 맵이 이동가능한 곳인가?\n(끝인지, 벽이있는지)
    (if _go
      (`self.SettingCharPos` _returnvalue _returnvalue_2))))

(fn `Update Logic`
  (switch `/Game/BluePrint/EnumStruct/EnumState` (`self.State`)
    (:`NewEnumerator1`
      (if (`self.ArrivedToDestination`)
        (`self.Update Destination`)
        (else
          (`self.AddMovementInput` (- (`self.CharcterPos`) (`self.K2_GetActorLocation`))) ; False : 목적지에 도달하지 \n못했을 시에 이동하기
        )))))

(fn `UserConstructionScript`)