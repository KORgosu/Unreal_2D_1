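; BP_SpawnMonsterPool keeps skeleton monsters populated on the BP_TileMap that owns it, up to a maximum creature count.
; On BeginPlay it caches the owning tile map and starts a self-calling spawn loop.
; Below the cap, the loop increments the count, waits a random delay, then has the tile map spawn a skeleton.
; At the cap it rechecks each tick, and DespawnCreatureCount decrements the count to free a slot.
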(event `self.ReceiveBeginPlay`
  (bind _asbp_tile_map (cast `/Game/BluePrint/BP_TileMap` (`self.GetOwner`)))
  (set `self.Tile Map` _asbp_tile_map)
  (`self.UpdateRandomSpawn`))

(event `UpdateRandomSpawn`
  (if (< (`self.CreatureCount`) (`self.MaxCreatureCount`))
    (`/Engine/EditorBlueprintResources/StandardMacros.IncrementInt` (`self.CreatureCount`)
      (:`  `
        (`KismetSystemLibrary.Delay` (`KismetMathLibrary.RandomFloatInRange` 0.0 10.0)) ; 조금의 딜레이를 거친 뒤
        (`/Game/BluePrint/BP_TileMap.SpawnMonster` (`self.Tile Map`) "/Game/BluePrint/Creatures/BP_Skeleton_Monster.BP_Skeleton_Monster_C") ; 몬스터를 스폰한다
        (`self.UpdateRandomSpawn`)))
    (else
      (`KismetSystemLibrary.DelayUntilNextTick`) ; 다음 틱까지 몬스터를 스폰하지 않고 대기
      (`self.UpdateRandomSpawn`) ; 재귀
    )))

(fn `DespawnCreatureCount`
  (`/Engine/EditorBlueprintResources/StandardMacros.DecrementInt` (`self.CreatureCount`)))