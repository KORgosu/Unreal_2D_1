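; 2D flipbook creature with four-way movement, a melee attack and health, using stats and animations from a Data asset.
; Each tick, State and Direction drive movement and flipbook choice, with side sprites rotated to mirror left.
; Attack_Begin damages other creatures overlapping the directional range, waits out the flipbook, then returns to Move.
; OnDamaged clamps HP and updates the HP bar widget; no death handling is present.
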(event `self.ReceiveBeginPlay`
  (bind _output_get (set `self.HP` (`.HPMAX_26_8AC06505446583406658AEB219CB0C5F` (break `/Game/BluePrint/DataTable/Creature_Data` (`self.Data`)))))
  (set `self.MaxHP` _output_get))

(event `self.ReceiveTick`
  (params (DeltaSeconds :type "Float (single-precision)"))
  (`self.Update Logic`)
  (`self.Update Animate`))

(event `Attack_Begin`
  (switch `/Game/BluePrint/EnumState` (`self.State`)
    (:`NewEnumerator0`
      _)
    (:`NewEnumerator1`
      _))
  (set `self.State` "NewEnumerator2")
  (`self.Update Animate`)
  (`self.Attack_Process`)
  (`KismetSystemLibrary.Delay` (`PaperFlipbookComponent.GetFlipbookLength` (`self.Sprite`)))
  (set `self.State` "NewEnumerator1"))

(fn `Attack_Process`
  (bind _attackrangeside (`self.AttackRangeSIDE`))
  (for _array_element (`PrimitiveComponent.GetOverlappingActors` (select `/Game/BluePrint/EnumDirection` (`self.Direction`) :`NewEnumerator0` (`self.AttackRangeUP`) :`NewEnumerator1` (`self.AttackRangeDOWN`) :`NewEnumerator2` _attackrangeside :`NewEnumerator3` _attackrangeside) "BP_Creature_C")
    (bind _asbp_creature (cast `/Game/BluePrint/BP_Creature` _array_element))
    (if (not (== _asbp_creature self))
      (`self.OnDamaged` _asbp_creature 10 self))))

(fn `OnDamaged`
  (params (Damage :type Integer) (Attack :type "/Game/BluePrint/BP_Creature Object Reference"))
  (bind _maxhp (`self.MaxHP`))
  (if (not (== Attack self))
    (bind _output_get (set `self.HP` (`KismetMathLibrary.Clamp` (- (`self.HP`) Damage) 0 _maxhp)))
    (bind _aswizet_bp_hp (cast `/Game/BluePrint/UI/WizetBP_HP` (`WidgetComponent.GetUserWidgetObject` (`self.HpBar`))))
    (set `/Game/BluePrint/UI/WizetBP_HP.HpRatio` (/ _output_get (`KismetMathLibrary.Conv_IntToDouble` _maxhp)) _aswizet_bp_hp)))

(fn `Update Animate`
  (bind (_data_hpmax _data_damage _data_up_idle _data_down_idle _data_side_idle _data_up_move _data_down_move _data_side_move _data_up_attack _data_down_attack _data_side_attack) (break `/Game/BluePrint/DataTable/Creature_Data` (`self.Data`)))
  (`SceneComponent.K2_SetRelativeRotation` (`self.Sprite`) (select `bool` (`|EnumEquality` (`self.Direction`) "NewEnumerator2") :`true` (struct :`Yaw` 180.0) :!type "Rotator Structure") false false)
  (switch `/Game/BluePrint/EnumState` (`self.State`)
    (:`NewEnumerator0`
      (`PaperFlipbookComponent.SetFlipbook` (`self.Sprite`) (select `/Game/BluePrint/EnumDirection` (`self.Direction`) :`NewEnumerator0` _data_up_idle :`NewEnumerator1` _data_down_idle :`NewEnumerator2` _data_side_idle :`NewEnumerator3` _data_side_idle)))
    (:`NewEnumerator1`
      (`PaperFlipbookComponent.SetFlipbook` (`self.Sprite`) (select `/Game/BluePrint/EnumDirection` (`self.Direction`) :`NewEnumerator0` _data_up_move :`NewEnumerator1` _data_down_move :`NewEnumerator2` _data_side_move :`NewEnumerator3` _data_side_move)))
    (:`NewEnumerator2`
      (`PaperFlipbookComponent.SetFlipbook` (`self.Sprite`) (select `/Game/BluePrint/EnumDirection` (`self.Direction`) :`NewEnumerator0` _data_up_attack :`NewEnumerator1` _data_down_attack :`NewEnumerator2` _data_side_attack :`NewEnumerator3` _data_side_attack)))))

(fn `Update Logic`
  (switch `/Game/BluePrint/EnumState` (`self.State`)
    (:`NewEnumerator1`
      (`self.AddMovementInput` (select `/Game/BluePrint/EnumDirection` (`self.Direction`) :`NewEnumerator0` (0.0 0.0 1.0) :`NewEnumerator1` (0.0 0.0 -1.0) :`NewEnumerator2` (-1.0 0.0 0.0) :`NewEnumerator3` (1.0 0.0 0.0) :!type "Vector Structure")))))

(fn `UserConstructionScript`)