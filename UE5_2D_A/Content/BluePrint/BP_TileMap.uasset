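; Tile map actor that serves as the grid board for a knight-versus-skeleton game, tracking walls and creatures.
; BeginPlay builds a blocked-cell array from tile layer 1 (assuming 10 columns), randomly places the existing knight, spawns two skeletons and adds the UI widget.
; Helpers convert grid coordinates to indices and X/Z world positions, check walkability against walls and creatures, pick random empty cells with capped retries, and despawn creatures.
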(event `self.ReceiveBeginPlay`
  (bind (_spawn_pos__x _spawn_pos__y) (break `/Game/BluePrint/EnumStruct/EnumGridPosition` (`self.GetEmptyGrid`)))
  (bind _tilemap (`PaperTileMapComponent.TileMap` (`self.RenderComponent`)))
  (bind _mapwidth (`PaperTileMap.MapWidth` _tilemap))
  (bind _mapheight (`PaperTileMap.MapHeight` _tilemap))
  (`|ExecutionSequence`
    (:`then_0`
      (`KismetArrayLibrary.Array_Resize` (`self.MapGrid`) (* _mapwidth _mapheight)) ; 맵 크기를 조절하는 과정
      (set `self.MapWidth` _mapwidth)
      (set `self.MapHeight` _mapheight))
    (:`then_1`
      (for (_ _array_index) (`self.MapGrid`)
        (bind (_returnvalue_tileindex _returnvalue_tileset) (break `PaperTileInfo` (`PaperTileMapComponent.GetTile` (`self.RenderComponent`) (mod _array_index 10) (/ _array_index 10) 1)))
        (`/Engine/EditorBlueprintResources/StandardMacros.IsValid` _returnvalue_tileset ; 벽 타일인지에 대한 여부
          (:`Is Valid`
            (`KismetArrayLibrary.Array_Set` (`self.MapGrid`) _array_index true)))))
    (:`then_2`
      (bind _returnvalue (`GameplayStatics.GetActorOfClass` "/Game/BluePrint/Creatures/BP_Knight.BP_Knight_C"))
      (`/Game/BluePrint/Creatures/BP_Creature.SettingCharPos` _returnvalue _spawn_pos__x _spawn_pos__y true) ; 랜덤위치에 캐릭터 소환
      (`KismetArrayLibrary.Array_Add` (`self.BP_Creature`) _returnvalue)
      (`self.SpawnMonster` "/Game/BluePrint/Creatures/BP_Skeleton_Monster.BP_Skeleton_Monster_C") ; 랜덤위치에 해골소환
      (`self.SpawnMonster` "/Game/BluePrint/Creatures/BP_Skeleton_Monster.BP_Skeleton_Monster_C") ; 랜덤위치에 해골소환
    )
    (:`then_3`
      (bind _returnvalue_2 (`|CreateWidget` "/Game/BluePrint/UI/WizetBP_UI.WizetBP_UI_C")) ; 킬수 표시
      (bind _output_get (set `self.GameUI` _returnvalue_2))
      (`UserWidget.AddToViewport` _output_get 0))))

(fn `DespawnMonster`
  (params (Creature :type "/Game/BluePrint/Creatures/BP_Creature Object Reference"))
  (`/Engine/EditorBlueprintResources/StandardMacros.IsValid` Creature
    (:`Is Valid`
      (`KismetArrayLibrary.Array_RemoveItem` (`self.BP_Creature`) Creature)
      (`self.K2_DestroyActor` Creature))))

(fn `GetCreatureAtGrid`
  (params (GridX :type Integer) (GridY :type Integer))
  (returns (isFound :type Boolean) (Creature :type "/Game/BluePrint/Creatures/BP_Creature Object Reference"))
  (for _array_element (`self.BP_Creature`)
    (bind (_gridpos_x _gridpos_y) (break `/Game/BluePrint/EnumStruct/EnumGridPosition` (`/Game/BluePrint/Creatures/BP_Creature.GridPos` _array_element)))
    (if (and (== _gridpos_x GridX) (== _gridpos_y GridY))
      (return true _array_element) ; 몬스터 발견한거
    ))
  (return false null) ; 몬스터 발견못함
)

(fn `GetEmptyGrid`
  (returns (`Spawn Pos ` :type "/Game/BluePrint/EnumStruct/EnumGridPosition Structure"))
  (locals (RandomPos :type "/Game/BluePrint/EnumStruct/EnumGridPosition Structure"))
  (for _ (range 1001)
    (bind _output_get (set `local.RandomPos` (make `/Game/BluePrint/EnumStruct/EnumGridPosition` (`KismetMathLibrary.RandomIntegerInRange` 0 (- (`self.MapWidth`) 1)) (`KismetMathLibrary.RandomIntegerInRange` 0 (- (`self.MapHeight`) 1)))))
    (bind _go (`self.Go` (break `/Game/BluePrint/EnumStruct/EnumGridPosition` _output_get) (`.Y_4_C21992ED433FA79B6561139056341895` (break `/Game/BluePrint/EnumStruct/EnumGridPosition` _output_get))))
    (if _go
      (break)))
  (return (`local.RandomPos`)) ; 최종 몬스터소환지역 RandomPos에 저장
)

(fn `GetWorldPos`
  (params (GridX :type Integer) (GridY :type Integer))
  (returns (Valid :type Boolean) (Pos :type "Vector Structure"))
  (bind _valid (`self.GridPos` GridX GridY))
  (return _valid (+ (`self.K2_GetActorLocation`) (`KismetMathLibrary.MakeVector` (* GridX (`self.WorldSize_X`) 5.0) 0.0 (* GridY (`self.WorldSize_Y`) -5.0)))))

(fn `Go`
  (params (X :type Integer) (Y :type Integer))
  (returns (Go :type Boolean))
  (bind (_valid _index) (`self.GridPos` X Y)) ; 해당위치가 유효한가?
  (if _valid
    (if (not (`|GetArrayItem` (`self.MapGrid`) _index))
      (bind _isfound (`self.GetCreatureAtGrid` X Y)) ; 해당 그리드에 creature가 존재한가? Found가 True면 못감
      (return (not _isfound))
      (else
        _)))
  (return false))

(fn `GridPos`
  (params (GridX :type Integer) (GridY :type Integer))
  (returns (Valid :type Boolean) (Index :type Integer))
  (bind _mapwidth (`self.MapWidth`))
  (return (and (`KismetMathLibrary.InRange_IntInt` GridX 0 _mapwidth) (`KismetMathLibrary.InRange_IntInt` GridY 0 (`self.MapHeight`))) (+ GridX (* GridY _mapwidth))))

(fn `SpawnMonster`
  (params (Class :type "/Game/BluePrint/Creatures/BP_Creature Class Reference"))
  (bind (_spawn_pos__x _spawn_pos__y) (break `/Game/BluePrint/EnumStruct/EnumGridPosition` (`self.GetEmptyGrid`)))
  (bind (_valid _pos) (`self.GetWorldPos` _spawn_pos__x _spawn_pos__y))
  (if _valid
    (bind _returnvalue (`|SpawnActorFromClass` Class (`KismetMathLibrary.MakeTransform` (`KismetMathLibrary.MakeVector` (.x _pos) 500.0 (.z _pos))) "Undefined" "OverrideRootScale" null null))
    (`/Game/BluePrint/Creatures/BP_Creature.SettingCharPos` _returnvalue _spawn_pos__x _spawn_pos__y true)
    (`KismetArrayLibrary.Array_Add` (`self.BP_Creature`) _returnvalue)))

(fn `UserConstructionScript`)